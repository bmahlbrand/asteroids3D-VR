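; Asteroid hazard that homes in on the player pawn while tumbling, with randomized speed and spin each tick.
; BeginPlay spawns an effect and randomizes mesh, material and one of three sizes, which sets health and point value.
; Overlap plays an explosion sound, damages the other actor and destroys the asteroid.
; Incoming damage spawns effects and reduces health; at zero, it adds points to the AsteroidsHUD score and destroys itself.
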(event OnComponentBeginOverlap(StaticMesh)
  (params (OtherActor :type Actor%20Object%20Reference) (OtherComp :type Primitive%20Component%20Object%20Reference) (OtherBodyIndex :type Integer) (bFromSweep :type Boolean) (SweepResult :type Hit%20Result%20Structure%20%28by%20ref%29))
  (Audio|PlaySoundatLocation "/Game/EpicsMobileStarterContent/Audio/Explosion02.Explosion02" "0, 0, 0")
  (Game|Damage|ApplyDamage OtherActor 1e+01 0 0 "/Script/Engine.DamageType")
  (Actor|DestroyActor))

(event EventBeginPlay
  (bind _asteroid (Variables|Default|GetAsteroid))
  (bind _asteroid_2 (Variables|Default|GetAsteroid))
  (Utilities|FlowControl|Sequence
    (:then_0
      (Effects|SpawnEmitteratLocation "/Game/Lesson2/Effects/P_Explosion_Orange2.P_Explosion_Orange2" (Transformation|GetActorLocation) "0, 0, 0" false))
    (:then_1
      (switch int (Math|Random|RandomInteger 3)
        (:Default
          (Components|StaticMesh|SetStaticMesh _asteroid "/Game/Lesson2/Meshes/Rock/SM_Asteroid_001.SM_Asteroid_001" :!label _label))
        (:0
          (goto _label))
        (:1
          (Components|StaticMesh|SetStaticMesh _asteroid "/Game/Lesson2/Meshes/Rock/SM_Asteroid_002.SM_Asteroid_002"))
        (:2
          (Components|StaticMesh|SetStaticMesh _asteroid "/Game/Lesson2/Meshes/Rock/SM_Asteroid_003.SM_Asteroid_003"))
        (:3
          (Components|StaticMesh|SetStaticMesh _asteroid "/Game/Lesson2/Meshes/Rock/SM_Asteroid_004.SM_Asteroid_004")))
      (switch int (Math|Random|RandomInteger 3)
        (:0
          (Rendering|Material|SetMaterial _asteroid_2 0 "/Game/Lesson2/Materials/Asteroids/MI_Asteroid_001.MI_Asteroid_001"))
        (:1
          (Rendering|Material|SetMaterial _asteroid_2 0 "/Game/Lesson2/Materials/Asteroids/MI_Asteroid_002.MI_Asteroid_002"))
        (:2
          (Rendering|Material|SetMaterial _asteroid_2 0 "/Game/Lesson2/Materials/Asteroids/MI_Asteroid_003.MI_Asteroid_003")))
      (switch int (Math|Random|RandomInteger 3)
        (:0
          (Transformation|SetActorScale3D "0.330000,0.330000,0.330000")
          (bind _output_get (Variables|Default|SetHealth 1e+01))
          (Variables|Default|SetPointValue (/ _output_get 2.0)))
        (:1
          (Transformation|SetActorScale3D "0.750000,0.750000,0.750000")
          (bind _output_get_2 (Variables|Default|SetHealth 2e+01))
          (Variables|Default|SetPointValue (/ _output_get_2 2.0)))
        (:2
          (Transformation|SetActorScale3D "1.500000,1.500000,1.500000")
          (bind _output_get_3 (Variables|Default|SetHealth 3e+01))
          (Variables|Default|SetPointValue (/ _output_get_3 2.0)))))))

(event EventTick
  (params (DeltaSeconds :type Float%20%28single-precision%29))
  (bind _returnvalue (Math|Random|RandomFloatinRange 25.0 1e+02))
  (bind _returnvalue_2 (Math|Random|RandomFloatinRange 2e+01 5e+01))
  (bind _returnvalue_3 (* DeltaSeconds _returnvalue))
  (bind _returnvalue_4 (* DeltaSeconds _returnvalue_2))
  (Utilities|FlowControl|Sequence
    (:then_0
      (Transformation|AddActorWorldOffset (* (* (Class|KismetMathLibrary|GetDirectionVector (Transformation|GetActorLocation) (Transformation|GetActorLocation (Game|Player|GetPlayerPawn 0))) (Math|Vector|MakeVector _returnvalue_3 _returnvalue_3 _returnvalue_3)) 5.0) true))
    (:then_1
      (Transformation|AddActorLocalRotation (Math|Rotator|MakeRotator _returnvalue_4 _returnvalue_4 _returnvalue_4) false false))))

(event Game|Damage|EventAnyDamage
  (params (Damage :type Float%20%28single-precision%29) (DamageType :type Damage%20Type%20Object%20Reference) (InstigatedBy :type Controller%20Object%20Reference) (DamageCauser :type Actor%20Object%20Reference))
  (bind _returnvalue (Transformation|GetActorLocation))
  (bind _output_get (Variables|Default|SetHealth (- (Variables|Default|GetHealth) Damage)))
  (if (<= _output_get 0.0)
    (Utilities|FlowControl|Sequence
      (:then_0
        (Effects|SpawnEmitteratLocation "/Game/Lesson2/Effects/P_Explosion_Fuchsia.P_Explosion_Fuchsia" _returnvalue))
      (:then_1
        (bind _asasteroids_hud (Utilities|Casting|CastToAsteroidsHUD (HUD|GetHUD (Game|GetPlayerController 0))))
        (Variables|/Game/Lesson2/Blueprints/AsteroidsHUD.AsteroidsHUD_C|Setscore _asasteroids_hud (+ (Variables|/Game/Lesson2/Blueprints/AsteroidsHUD.AsteroidsHUD_C|Getscore _asasteroids_hud) (Variables|Default|GetPointValue))))
      (:then_2
        (Actor|DestroyActor)))
    (else
      (Effects|SpawnEmitteratLocation "/Game/Lesson2/Effects/P_Explosion_Fuchsia2.P_Explosion_Fuchsia2" _returnvalue))))

(fn ConstructionScript)