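; VR player Blueprint that highlights what the camera looks at and fires bullets.
; A looping timer runs a camera line trace, toggling Render Custom Depth on the hit static mesh and switching it off on the previous target.
; Space bar spawns a BP_Bullet just ahead of the VR camera along its forward vector.
; An overlap on the Sphere component plays an explosion sound at the actor's location.
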(event OnComponentBeginOverlap(Sphere)
  (params (OtherActor :type Actor%20Object%20Reference) (OtherComp :type Primitive%20Component%20Object%20Reference) (OtherBodyIndex :type Integer) (bFromSweep :type Boolean) (SweepResult :type Hit%20Result%20Structure%20%28by%20ref%29))
  (Audio|PlaySoundatLocation "/Game/MobileStarterContent/Audio/Explosion_Cue.Explosion_Cue" (Transformation|GetActorLocation)))

(event EventBeginPlay
  (Utilities|Time|SetTimerbyFunctionName 0 "Trace" 0.1 true)
  (Development|PrintString "Hello"))

(event Input|KeyboardEvents|SpaceBar
  (params (Key :type Key%20Structure :default "AnyKey"))
  (:Pressed
    (CallFunction|ShootBullet)))

(fn ConstructionScript)

(fn ShootBullet
  (bind (_location _forward_vector) (CallFunction|GetPlayerVRCameraProperties))
  (Game|SpawnActorfromClass "/Game/Lesson2/Blueprints/BP_Bullet.BP_Bullet_C" (Math|Transform|MakeTransform (+ _location (* _forward_vector 60)) (Math|Conversions|RotationFromXVector _forward_vector)) "Undefined" 0 0)
  (return))

(fn Trace
  (bind _camera (Variables|Default|GetCamera))
  (bind _returnvalue (Transformation|GetWorldLocation _camera))
  (bind (_outhit _returnvalue_2) (Collision|LineTraceByChannel _returnvalue (+ _returnvalue (* (Math|Vector|GetForwardVector (.Rotation (Math|Transform|BreakTransform (Transformation|GetWorldTransform (Variables|Default|GetCamera))))) 1e+04)) "TraceTypeQuery1" false 0 "None"))
  (if _returnvalue_2
    (bind _asstatic_mesh_component (Utilities|Casting|CastToStaticMeshComponent (.HitComponent (Collision|BreakHitResult _outhit)))
      (:then
        (if (== _asstatic_mesh_component (Variables|Default|GetCurrent%20Target))
          _
          (else
            (Rendering|SetRenderCustomDepth (Variables|Default|GetCurrent%20Target) false)))
        (Variables|Default|SetCurrent%20Target _asstatic_mesh_component)
        (Rendering|SetRenderCustomDepth _asstatic_mesh_component true))
      (:CastFailed
        (Utilities|IsValid (Variables|Default|GetCurrent%20Target) :!label _label
          (:Is%20Valid
            (Rendering|SetRenderCustomDepth (Variables|Default|GetCurrent%20Target) false)
            (Variables|Default|SetCurrent%20Target (Variables|Default|GetCurrent%20Target))))))
    (else
      (goto _label))))