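; BP_Asteroid is a destructible asteroid actor that homes in on the player pawn while tumbling.
; BeginPlay randomizes its mesh, material and scale, with Health tied to the chosen size.
; Tick moves it toward player 0 with a swept offset and applies jittered local rotation.
; AnyDamage reduces Health, then spawns an explosion and destroys the actor at zero; the PointValue scoring logic is unconnected.
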(event EventBeginPlay
  (bind _asteroid (Variables|Default|GetAsteroid))
  (bind _asteroid_2 (Variables|Default|GetAsteroid))
  (Utilities|FlowControl|Sequence
    (:then_1
      (switch int (Math|Random|RandomInteger 3)
        (:Default
          (Components|StaticMesh|SetStaticMesh _asteroid "/Game/Lesson2/Meshes/Rock/SM_Asteroid_001.SM_Asteroid_001" :!label _label))
        (:0
          (goto _label))
        (:1
          (Components|StaticMesh|SetStaticMesh _asteroid "/Game/Lesson2/Meshes/Rock/SM_Asteroid_002.SM_Asteroid_002"))
        (:2
          (Components|StaticMesh|SetStaticMesh _asteroid "/Game/Lesson2/Meshes/Rock/SM_Asteroid_003.SM_Asteroid_003"))
        (:3
          (Components|StaticMesh|SetStaticMesh _asteroid "/Game/Lesson2/Meshes/Rock/SM_Asteroid_004.SM_Asteroid_004")))
      (switch int (Math|Random|RandomInteger 2)
        (:0
          (Rendering|Material|SetMaterial _asteroid_2 0 "/Game/Lesson2/Materials/Asteroids/MI_Asteroid_001.MI_Asteroid_001"))
        (:1
          (Rendering|Material|SetMaterial _asteroid_2 0 "/Game/Lesson2/Materials/Asteroids/MI_Asteroid_002.MI_Asteroid_002"))
        (:2
          (Rendering|Material|SetMaterial _asteroid_2 0 "/Game/Lesson2/Materials/Asteroids/MI_Asteroid_003.MI_Asteroid_003")))
      (switch int (Math|Random|RandomInteger 2)
        (:0
          (Transformation|SetActorScale3D "0.330000,0.330000,0.330000")
          (Variables|Default|SetHealth 1e+01))
        (:1
          (Transformation|SetActorScale3D "0.750000,0.750000,0.750000")
          (Variables|Default|SetHealth 2e+01))
        (:2
          (Transformation|SetActorScale3D "1.500000,1.500000,1.500000")
          (Variables|Default|SetHealth 3e+01))))))

(event EventTick
  (params (DeltaSeconds :type Float%20%28single-precision%29))
  (bind _returnvalue (Math|Random|RandomFloatinRange 2e+01 5e+01))
  (bind _returnvalue_2 (* DeltaSeconds 75.0))
  (bind _returnvalue_3 (* DeltaSeconds _returnvalue))
  (Utilities|FlowControl|Sequence
    (:then_0
      (Transformation|AddActorWorldOffset (* (* (Class|KismetMathLibrary|GetDirectionVector (Transformation|GetActorLocation) (Transformation|GetActorLocation (Game|Player|GetPlayerPawn 0))) (Math|Vector|MakeVector _returnvalue_2 _returnvalue_2 _returnvalue_2)) 5.0) true))
    (:then_1
      (Transformation|AddActorLocalRotation (Math|Rotator|MakeRotator _returnvalue_3 _returnvalue_3 _returnvalue_3) false false))))

(event Game|Damage|EventAnyDamage
  (params (Damage :type Float%20%28single-precision%29) (DamageType :type Damage%20Type%20Object%20Reference) (InstigatedBy :type Controller%20Object%20Reference) (DamageCauser :type Actor%20Object%20Reference))
  (Development|PrintString "damage received")
  (bind _output_get (Variables|Default|SetHealth (- (Variables|Default|GetHealth) Damage)))
  (if (<= _output_get 0.0)
    (Utilities|FlowControl|Sequence
      (:then_0
        (Effects|SpawnEmitteratLocation "/Game/MobileStarterContent/Particles/P_Explosion.P_Explosion" (Transformation|GetActorLocation))
        (Actor|DestroyActor)))))

(fn ConstructionScript)