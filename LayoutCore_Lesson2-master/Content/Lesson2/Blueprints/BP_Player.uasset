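; BP_Player is a player Blueprint that shoots bullets from the VR camera and sounds an explosion when something overlaps it.
; Pressing Space calls ShootBullet, which spawns a BP_Bullet slightly ahead of the VR camera, oriented along its forward vector.
; Its Sphere component's begin overlap plays the explosion cue at the actor's location, with no damage or other response.
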(event OnComponentBeginOverlap(Sphere)
  (params (OtherActor :type Actor%20Object%20Reference) (OtherComp :type Primitive%20Component%20Object%20Reference) (OtherBodyIndex :type Integer) (bFromSweep :type Boolean) (SweepResult :type Hit%20Result%20Structure%20%28by%20ref%29))
  (Audio|PlaySoundatLocation "/Game/MobileStarterContent/Audio/Explosion_Cue.Explosion_Cue" (Transformation|GetActorLocation)))

(event EventBeginPlay)

(event EventActorBeginOverlap
  (params (OtherActor :type Actor%20Object%20Reference)))

(event EventTick
  (params (DeltaSeconds :type Float%20%28single-precision%29)))

(event Input|KeyboardEvents|SpaceBar
  (params (Key :type Key%20Structure :default "AnyKey"))
  (:Pressed
    (CallFunction|ShootBullet)))

(fn ConstructionScript)

(fn ShootBullet
  (bind (_location _forward_vector) (CallFunction|GetPlayerVRCameraProperties))
  (Game|SpawnActorfromClass "/Game/Lesson2/Blueprints/BP_Bullet.BP_Bullet_C" (Math|Transform|MakeTransform (+ _location (* _forward_vector 60)) (Math|Conversions|RotationFromXVector _forward_vector)) "Undefined" 0 0)
  (return))